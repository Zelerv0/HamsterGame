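; Game mode for 1v1 matches that registers joining players by team and places them at team spawn points.
; The construction script sorts spawn points into red and blue arrays.
; On login it initializes team UI, registers the player with GS_1v1, copies team to the controller and sets DefaultPawnClass from their selected character.
; ChoosePlayerStart steps through the team's array with a counter, while FindPlayerStart picks one randomly.
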(event `self.K2_PostLogin`
  (params (NewPlayer :type "PlayerController Object Reference"))
  (bind _playerstate (`Controller.PlayerState` NewPlayer))
  (bind _asbp_1v_1player_state (cast `/Game/BluePrints/PlayerState/BP_1v1PlayerState` _playerstate :!pure true))
  (`/Game/BluePrints/Character/BP_Base_PlayerController.InishalizeTeamsUI` (cast `/Game/BluePrints/Character/BP_Base_PlayerController` (`PlayerState.GetPlayerController` _playerstate) :!pure true))
  (bind _asgs_1v_1 (cast `/Game/BluePrints/GameState/GS_1v1` (`GameplayStatics.GetGameState`)))
  (`/Game/BluePrints/GameState/GS_1v1.AddNewPlayer` _asgs_1v_1 (`AdvancedSessionsLibrary.GetUniqueNetIDFromPlayerState` _asbp_1v_1player_state) (`/Game/BluePrints/PlayerState/BP_1v1PlayerState.IsOnRedTeam` _asbp_1v_1player_state) _asbp_1v_1player_state)
  (bind _asbp_base_player_controller (cast `/Game/BluePrints/Character/BP_Base_PlayerController` (`PlayerState.GetPlayerController` _asbp_1v_1player_state)))
  (set `/Game/BluePrints/Character/BP_Base_PlayerController.IsRedPlayer` (`/Game/BluePrints/PlayerState/BP_1v1PlayerState.IsOnRedTeam` _asbp_1v_1player_state) _asbp_base_player_controller)
  (set `self.DefaultPawnClass` (`/Game/BluePrints/PlayerState/BP_1v1PlayerState.SelectedCharacter` _asbp_1v_1player_state)))

(event `self.ReceiveBeginPlay`)

(fn `ChoosePlayerStart`
  (params (Player :type "Controller Object Reference"))
  (returns (ReturnValue :type "Actor Object Reference"))
  (bind _asbp_base_player_controller (cast `/Game/BluePrints/Character/BP_Base_PlayerController` Player))
  (if (`/Game/BluePrints/Character/BP_Base_PlayerController.IsRedPlayer` _asbp_base_player_controller)
    (bind _result (`/Engine/EditorBlueprintResources/StandardMacros.IncrementInt` (`self.NextRedPlayerStartIndext`))
      (:`  `
        (return (`|GetArrayItem` (`self.RedTeamSpawn`) _result))))
    (else
      (bind _result_2 (`/Engine/EditorBlueprintResources/StandardMacros.IncrementInt` (`self.NextBluePlayerStartIndext`))
        (:`  `
          (return (`|GetArrayItem` (`self.BlueTeamSpawn`) _result_2)))))))

(fn `FindPlayerStart`
  (params (Player :type "Controller Object Reference") (IncomingName :type String))
  (returns (ReturnValue :type "Actor Object Reference"))
  (bind _asbp_base_player_controller (cast `/Game/BluePrints/Character/BP_Base_PlayerController` Player))
  (if (`/Game/BluePrints/Character/BP_Base_PlayerController.IsRedPlayer` _asbp_base_player_controller)
    (return (`|GetArrayItem` (`self.RedTeamSpawn`) (`KismetMathLibrary.RandomIntegerInRange` 0 (- (`KismetArrayLibrary.Array_Length` (`self.RedTeamSpawn`)) 1))))
    (else
      (return (`|GetArrayItem` (`self.BlueTeamSpawn`) (`KismetMathLibrary.RandomIntegerInRange` 0 (- (`KismetArrayLibrary.Array_Length` (`self.BlueTeamSpawn`)) 1)))))))

(fn `UserConstructionScript`
  (bind _outactors (`GameplayStatics.GetAllActorsOfClass` "/Game/BluePrints/Character/PlayerStart/PS_SpawnPoint.PS_SpawnPoint_C"))
  (for _array_element _outactors
    (if (`/Game/BluePrints/Character/PlayerStart/PS_SpawnPoint.IsRedTeam` _array_element)
      (`KismetArrayLibrary.Array_Add` (`self.RedTeamSpawn`) _array_element)
      (else
        (`KismetArrayLibrary.Array_Add` (`self.BlueTeamSpawn`) _array_element)))))