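; Lobby game mode that tracks joining and leaving players and sends the session to a map.
; PostLogin registers each player state with GS_Lobby, refreshes player info, stores the unique net ID and raises the player count.
; OnLogout removes the net ID and lowers the count.
; SendToMap performs a server travel on authority, and CallReadyButtons triggers a ready-button update with a debug print.
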(event `SendToMap`
  (params (MapPath :type String))
  (`/Engine/EditorBlueprintResources/ActorMacros.Switch Has Authority`
    (:`Authority`
      (`AdvancedSessionsLibrary.ServerTravel` MapPath))))

(event `self.K2_PostLogin`
  (params (NewPlayer :type "PlayerController Object Reference"))
  (bind _asgs_lobby (cast `/Game/BluePrints/GameState/GS_Lobby` (`GameplayStatics.GetGameState`)))
  (`/Game/BluePrints/GameState/GS_Lobby.AddPlayerToList` _asgs_lobby (cast `/Game/BluePrints/PlayerState/BP_PlayerStateLobby` (`Controller.PlayerState` NewPlayer) :!pure true))
  (`/Game/BluePrints/GameState/GS_Lobby.UpdateInfoPlayers` _asgs_lobby)
  (`KismetArrayLibrary.Array_Add` (`self.Unique Net Id`) (`AdvancedSessionsLibrary.GetUniqueNetID` NewPlayer))
  (bind _asgs_lobby_2 (cast `/Game/BluePrints/GameState/GS_Lobby` (`GameplayStatics.GetGameState`)))
  (set `/Game/BluePrints/GameState/GS_Lobby.AmountOfPlayers` (+ (`/Game/BluePrints/GameState/GS_Lobby.AmountOfPlayers` _asgs_lobby_2) 1) _asgs_lobby_2))

(event `self.K2_OnLogout`
  (params (ExitingController :type "Controller Object Reference"))
  (bind _asplayer_controller (cast `PlayerController` ExitingController))
  (`KismetArrayLibrary.Array_RemoveItem` (`self.Unique Net Id`) (`AdvancedSessionsLibrary.GetUniqueNetID` _asplayer_controller))
  (bind _asgs_lobby (cast `/Game/BluePrints/GameState/GS_Lobby` (`GameplayStatics.GetGameState`)))
  (`/Engine/EditorBlueprintResources/StandardMacros.DecrementInt` (`/Game/BluePrints/GameState/GS_Lobby.AmountOfPlayers` _asgs_lobby)))

(fn `CallReadyButtons`
  (`self.UpdateReadyButtons`)
  (`KismetSystemLibrary.PrintString` "Called update ready buttons"))

(fn `UserConstructionScript`)