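; BP_ObjectPool is an object pool actor that spawns and stores instances of a given actor class.
; InitialPool saves the class and pre-spawns actors at the pool's transform in a loop bounded by ObjectCount, adding each to PoolOfObj.
; AddToPool grows the pool by spawning another instance of the saved class and incrementing ObjectCount.
; The Blueprint itself contains no logic for retrieving, deactivating or recycling pooled actors.
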(event `InitialPool`
  (params (ActorInPool :type "Actor Class Reference"))
  (set `self.ActorInPool` ActorInPool)
  (for _ (range (+ (`self.ObjectCount`) 1))
    (bind _returnvalue (`|SpawnActorFromClass` ActorInPool (`self.GetTransform` self) "Undefined" "MultiplyWithRoot" null null))
    (`KismetArrayLibrary.Array_AddUnique` (`self.PoolOfObj`) _returnvalue)))

(event `AddToPool`
  (bind _returnvalue (`|SpawnActorFromClass` (`self.ActorInPool`) (`self.GetTransform` self) "Undefined" "MultiplyWithRoot" null null))
  (`KismetArrayLibrary.Array_AddUnique` (`self.PoolOfObj`) _returnvalue)
  (`/Engine/EditorBlueprintResources/StandardMacros.IncrementInt` (`self.ObjectCount`)))

(fn `UserConstructionScript`)