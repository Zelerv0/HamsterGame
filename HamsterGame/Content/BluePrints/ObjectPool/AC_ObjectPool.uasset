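; Actor component that keeps a pool of pre-spawned actors for reuse.
; InitialPool stores the actor class and owner, then spawns the starting batch into PoolOfObj.
; FindFirstAvailable returns the first BP_PooledObject flagged IsAvailable; when none is free, it calls AddToPool and searches again.
; AddToPool grows the pool by one actor, spawning only on the authority.
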(event `InitialPool`
  (params (ActorInPool :type "Actor Class Reference") (Owner :type "Actor Object Reference"))
  (bind _output_get (set `self.Owner` Owner))
  (bind _output_get_2 (set `self.ActorInPool` ActorInPool))
  (for _ (range (+ (`self.ObjectCount`) 1))
    (bind _returnvalue (`|SpawnActorFromClass` _output_get_2 (`KismetMathLibrary.MakeTransform` (1000.0 1000.0 100.0)) "Undefined" "MultiplyWithRoot" _output_get null))
    (`KismetArrayLibrary.Array_AddUnique` (`self.PoolOfObj`) _returnvalue)))

(event `AddToPool`
  (`/Engine/EditorBlueprintResources/ActorComponentMacros.Switch Has Authority`
    (:`Authority`
      (bind _returnvalue (`|SpawnActorFromClass` (`self.ActorInPool`) (`KismetMathLibrary.MakeTransform` (0.0 0.0 100.0)) "Undefined" "MultiplyWithRoot" (`self.Owner`) null))
      (`KismetArrayLibrary.Array_AddUnique` (`self.PoolOfObj`) _returnvalue)
      (`/Engine/EditorBlueprintResources/StandardMacros.IncrementInt` (`self.ObjectCount`)))))

(fn `FindFirstAvailable`
  (returns (`AsBP Pooled Object` :type "/Game/BluePrints/ObjectPool/BP_PooledObject Object Reference"))
  (locals (i :type Integer))
  (bind _poolofobj (`self.PoolOfObj`))
  (for _array_element _poolofobj :!label _label
    (bind _asbp_pooled_object (cast `/Game/BluePrints/ObjectPool/BP_PooledObject` _array_element))
    (if (`/Game/BluePrints/ObjectPool/BP_PooledObject.IsAvailable` _asbp_pooled_object)
      (return _asbp_pooled_object)
      (else
        (`/Engine/EditorBlueprintResources/StandardMacros.IncrementInt` (`local.i`)))))
  (if (== (`local.i`) (`KismetArrayLibrary.Array_Length` _poolofobj))
    (`self.AddToPool`)
    (set `local.i` 0)
    (goto _label)
    (else
      (set `local.i` 0))))