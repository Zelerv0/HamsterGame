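; Pooled projectile actor that is reused by toggling availability, visibility and sphere collision.
; SetProjectileAvailable applies a transform facing the stored direction, sets the owner, enables collision and starts a lifetime timer, while separate events set direction and movement speed.
; A hit or timer expiry calls HideObject, which frees it, disables collision and zeroes speed limits.
; Visibility replicates through a RepNotify with forced net updates.
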(event `self.ReceiveBeginPlay`
  (`PrimitiveComponent.SetCollisionEnabled` (`self.Sphere`) "NoCollision"))

(event `self.ProjectileMovement.OnComponentActivated`
  (params (Component :type "ActorComponent Object Reference") (bReset :type Boolean))
  (bind _projectilemovement (`self.ProjectileMovement`))
  (set `ProjectileMovementComponent.InitialSpeed` 0.0 _projectilemovement)
  (set `ProjectileMovementComponent.MaxSpeed` 0.0 _projectilemovement))

(event `self.ReceiveHit`
  (params (MyComp :type "PrimitiveComponent Object Reference") (Other :type "Actor Object Reference") (OtherComp :type "PrimitiveComponent Object Reference") (bSelfMoved :type Boolean) (HitLocation :type "Vector Structure") (HitNormal :type "Vector Structure") (NormalImpulse :type "Vector Structure") (Hit :type "HitResult Structure (by ref)"))
  (`self.HideObject`))

(event `SetProjectileAvailable`
  (params (ActorForTransform :type "Actor Object Reference") (NewTransform :type "Transform Structure (by ref)") (NewOwner :type "Actor Object Reference"))
  (set `self.IsAvailable` false)
  (set `self.IsVisible` true)
  (`self.ForceNetUpdate`)
  (`self.K2_SetActorTransform` ActorForTransform (`KismetMathLibrary.MakeTransform` NewTransform_Location (`KismetMathLibrary.MakeRotFromX` (`self.Direction`))) false false)
  (`PrimitiveComponent.SetCollisionEnabled` (`self.Sphere`) "QueryAndPhysics")
  (`self.SetOwner` NewOwner)
  (`KismetSystemLibrary.K2_SetTimerDelegate` (delegate `DeactivateObject`) (`self.LifeTime`)))

(event `DeactivateObject`
  (if (not (`self.IsAvailable`))
    (`self.HideObject`)))

(event `SetProjectileDirection`
  (params (StartPosition :type "Vector Structure") (EndPosition :type "Vector Structure") (Speed :type "Float (double-precision)"))
  (set `self.Direction` (* (`KismetMathLibrary.Normal` (- EndPosition StartPosition)) Speed)))

(event `SetProjectileSpeed`
  (params (`Initial Speed` :type "Float (single-precision)") (MaxSpeed :type "Float (single-precision)"))
  (bind _projectilemovement (`self.ProjectileMovement`))
  (set `ProjectileMovementComponent.InitialSpeed` `Initial Speed` _projectilemovement)
  (set `ProjectileMovementComponent.MaxSpeed` MaxSpeed _projectilemovement)
  (set `MovementComponent.Velocity` (`self.Direction`) _projectilemovement))

(fn `HideObject`
  (bind _projectilemovement (`self.ProjectileMovement`))
  (set `self.IsAvailable` true)
  (set `self.IsVisible` false)
  (`self.ForceNetUpdate`)
  (`PrimitiveComponent.SetCollisionEnabled` (`self.Sphere`) "NoCollision")
  (set `ProjectileMovementComponent.InitialSpeed` 0.0 _projectilemovement)
  (set `ProjectileMovementComponent.MaxSpeed` 0.0 _projectilemovement))

(fn `OnRep_IsVisible`
  (`self.SetActorHiddenInGame` (not (`self.IsVisible`))))

(fn `UserConstructionScript`)