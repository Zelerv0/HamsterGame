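; Base player controller that sets up Enhanced Input and the player HUD, then relays input to the possessed BP_BasePlayerPawn.
; BeginPlay adds the IM_Inputs mapping context, caches the cast pawn and creates the W_PlayerUI widget.
; Input events call pawn handlers for look, RPC-based move and jump, pause, two abilities, shoot and reload.
; The grapple input toggles, cancelling when a hook actor exists and firing otherwise.
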(event `self.ReceiveBeginPlay`
  (bind _returnvalue (pcsubsystem `EnhancedInputLocalPlayerSubsystem` self))
  (`/Engine/EditorBlueprintResources/StandardMacros.IsValid` _returnvalue
    (:`Is Valid`
      (`EnhancedInputSubsystemInterface.AddMappingContext` _returnvalue "/Game/BluePrints/Inputs/IM_Inputs.IM_Inputs" 0 (struct))
      (bind _output_get (set `self.ControlledPlayer` (`self.K2_GetPawn`)))
      (bind _asbp_base_player_pawn (cast `/Game/BluePrints/Character/BP_BasePlayerPawn` _output_get))
      (set `self.As BP Base Player Pawn` _asbp_base_player_pawn)
      (bind _returnvalue_2 (`|CreateWidget` "/Game/BluePrints/Widgets/W_PlayerUI.W_PlayerUI_C" self))
      (bind _output_get_2 (set `self.PlayerUIWidgetRef` _returnvalue_2))
      (`UserWidget.AddToViewport` _output_get_2 0))))

(event `EnhancedInput|/Game/BluePrints/Inputs/Keys/Actions_Movement/IA_LookXY`
  (params (ActionValue :type "Vector2D Structure") (ElapsedSeconds :type "Float (double-precision)") (TriggeredSeconds :type "Float (double-precision)") (InputAction :type "InputAction Object Reference" :default "/Game/BluePrints/Inputs/Keys/Actions_Movement/IA_LookXY.IA_LookXY"))
  ; Player base movement
  (:`Triggered`
    (`/Game/BluePrints/Character/BP_BasePlayerPawn.OnLookInput` (`self.As BP Base Player Pawn`) ActionValue_X ActionValue_Y)))

(event `EnhancedInput|/Game/BluePrints/Inputs/Keys/Actions_Movement/IA_Move`
  (params (ActionValue :type "Vector2D Structure") (ElapsedSeconds :type "Float (double-precision)") (TriggeredSeconds :type "Float (double-precision)") (InputAction :type "InputAction Object Reference" :default "/Game/BluePrints/Inputs/Keys/Actions_Movement/IA_Move.IA_Move"))
  ; Player base movement
  (:`Triggered`
    (`/Game/BluePrints/Character/BP_BasePlayerPawn.RPC_OnMoveInput` (`self.As BP Base Player Pawn`) ActionValue_X ActionValue_Y)))

(event `EnhancedInput|/Game/BluePrints/Inputs/Keys/Actions_Movement/IA_Jump`
  (params (ActionValue :type Boolean) (ElapsedSeconds :type "Float (double-precision)") (TriggeredSeconds :type "Float (double-precision)") (InputAction :type "InputAction Object Reference" :default "/Game/BluePrints/Inputs/Keys/Actions_Movement/IA_Jump.IA_Jump"))
  ; Player base movement
  (:`Started`
    (`/Game/BluePrints/Character/BP_BasePlayerPawn.RPC_OnJumpInput` (`self.As BP Base Player Pawn`))))

(event `EnhancedInput|/Game/BluePrints/Inputs/Keys/IA_Pause`
  (params (ActionValue :type Boolean) (ElapsedSeconds :type "Float (double-precision)") (TriggeredSeconds :type "Float (double-precision)") (InputAction :type "InputAction Object Reference" :default "/Game/BluePrints/Inputs/Keys/IA_Pause.IA_Pause"))
  ; Player UI interaction
  (:`Started`
    (`/Game/BluePrints/Character/BP_BasePlayerPawn.OnPauseInput` (`self.As BP Base Player Pawn`))))

(event `EnhancedInput|/Game/BluePrints/Inputs/Keys/Actions_Abilities/IA_Ability1`
  (params (ActionValue :type Boolean) (ElapsedSeconds :type "Float (double-precision)") (TriggeredSeconds :type "Float (double-precision)") (InputAction :type "InputAction Object Reference" :default "/Game/BluePrints/Inputs/Keys/Actions_Abilities/IA_Ability1.IA_Ability1"))
  ; Abilities
  (:`Started`
    (`/Game/BluePrints/Character/BP_BasePlayerPawn.OnAbility1Input` (`self.As BP Base Player Pawn`))))

(event `EnhancedInput|/Game/BluePrints/Inputs/Keys/Actions_Abilities/IA_Ability2`
  (params (ActionValue :type Boolean) (ElapsedSeconds :type "Float (double-precision)") (TriggeredSeconds :type "Float (double-precision)") (InputAction :type "InputAction Object Reference" :default "/Game/BluePrints/Inputs/Keys/Actions_Abilities/IA_Ability2.IA_Ability2"))
  ; Abilities
  (:`Started`
    (`/Game/BluePrints/Character/BP_BasePlayerPawn.OnAbility2Input` (`self.As BP Base Player Pawn`))))

(event `EnhancedInput|/Game/BluePrints/Inputs/Keys/Actions_Shooting/IA_Shoot`
  (params (ActionValue :type Boolean) (ElapsedSeconds :type "Float (double-precision)") (TriggeredSeconds :type "Float (double-precision)") (InputAction :type "InputAction Object Reference" :default "/Game/BluePrints/Inputs/Keys/Actions_Shooting/IA_Shoot.IA_Shoot"))
  (:`Triggered`
    (`/Game/BluePrints/Character/BP_BasePlayerPawn.OnShootInput` (`self.As BP Base Player Pawn`))))

(event `EnhancedInput|/Game/BluePrints/Inputs/Keys/Actions_Shooting/IA_Reload`
  (params (ActionValue :type Boolean) (ElapsedSeconds :type "Float (double-precision)") (TriggeredSeconds :type "Float (double-precision)") (InputAction :type "InputAction Object Reference" :default "/Game/BluePrints/Inputs/Keys/Actions_Shooting/IA_Reload.IA_Reload"))
  (:`Started`
    (`/Game/BluePrints/Character/BP_BasePlayerPawn.OnReloadInput` (`self.As BP Base Player Pawn`))))

(event `EnhancedInput|/Game/BluePrints/Inputs/Keys/Actions_Grapple/IA_Grapple`
  (params (ActionValue :type Boolean) (ElapsedSeconds :type "Float (double-precision)") (TriggeredSeconds :type "Float (double-precision)") (InputAction :type "InputAction Object Reference" :default "/Game/BluePrints/Inputs/Keys/Actions_Grapple/IA_Grapple.IA_Grapple"))
  (bind _as_bp_base_player_pawn (`self.As BP Base Player Pawn`))
  (:`Started`
    (`/Engine/EditorBlueprintResources/StandardMacros.IsValid` (`/Game/BluePrints/Character/BP_BasePlayerPawn.GrappleHookActor` (`self.As BP Base Player Pawn`))
      (:`Is Valid`
        (`/Game/BluePrints/Character/BP_BasePlayerPawn.CancelGrapple` _as_bp_base_player_pawn))
      (:`Is Not Valid`
        (`/Game/BluePrints/Character/BP_BasePlayerPawn.OnGrappleInput` _as_bp_base_player_pawn)))))

(fn `UserConstructionScript`)