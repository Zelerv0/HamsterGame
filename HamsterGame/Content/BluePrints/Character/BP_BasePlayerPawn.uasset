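; Base player pawn for a physics-driven beach ball that rolls, jumps and looks around.
; Input applies camera-relative velocity-correction forces to the Sphere below a speed threshold, while Tick traces for "Ground"-tagged actors to gate jump impulses and extra gravity.
; The BeachBall spins with horizontal speed as its Billboard slerps toward travel direction.
; MouseSave supplies look sensitivity and inversion, pause toggles W_Options, and jump buffering is left unwired.
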(event `self.ReceiveTick`
  (params (DeltaSeconds :type "Float (single-precision)"))
  (bind (_returnvalue_x _returnvalue_y) (`KismetMathLibrary.BreakVector` (`self.GetVelocity`)))
  (bind (_returnvalue_x_2 _returnvalue_y_2) (`KismetMathLibrary.BreakVector` (`self.GetVelocity`)))
  (bind (_returnvalue_roll _returnvalue_pitch _returnvalue_yaw) (`KismetMathLibrary.BreakRotator` (`KismetMathLibrary.Quat_Rotator` (`KismetMathLibrary.Quat_Slerp` (`KismetMathLibrary.Conv_RotatorToQuaternion` (`KismetMathLibrary.Conv_VectorToRotator` (`KismetMathLibrary.Normal` (`KismetMathLibrary.GetForwardVector` (`SceneComponent.RelativeRotation` (`self.Billboard`)))))) (`KismetMathLibrary.Conv_RotatorToQuaternion` (`KismetMathLibrary.Conv_VectorToRotator` (`KismetMathLibrary.Normal` (`self.GetVelocity`)))) 0.07))))
  (set `self.Delta Seconds` DeltaSeconds)
  (`|ExecutionSequence`
    (:`then_0`
      (`SceneComponent.K2_AddLocalRotation` (`self.BeachBall`) (`KismetMathLibrary.MakeRotator` 0.0 (* (`self.Delta Seconds`) (`self.Rotation Speed`) (`KismetMathLibrary.VSize` (`KismetMathLibrary.MakeVector` _returnvalue_x _returnvalue_y)))) false false)
      (if (>= (`KismetMathLibrary.VSize` (`KismetMathLibrary.MakeVector` _returnvalue_x_2 _returnvalue_y_2)) (`self.Rotation Threshold`))
        (`SceneComponent.K2_SetRelativeRotation` (`self.Billboard`) (`KismetMathLibrary.MakeRotator` 0.0 0.0 _returnvalue_yaw) false false)))
    (:`then_1`
      (`self.CheckGrounded`)
      (`self.SimulateGravity`)
      (if (`self.JumpBuffered`)
        (bind _output_get (set `self.JumpBuffer` (- (`self.JumpBuffer`) (`self.Delta Seconds`))))
        (if (<= _output_get 0.0)
          (set `self.JumpBuffered` false))))))

(event `self.ReceiveBeginPlay`
  (bind _returnvalue (`GameplayStatics.DoesSaveGameExist` (`self.Mouse Save Slot`)))
  (if _returnvalue
    (bind _returnvalue_2 (`GameplayStatics.LoadGameFromSlot` (`self.Mouse Save Slot`)))
    (bind _asmouse_save (cast `/Game/BluePrints/Saves/MouseSave` _returnvalue_2))
    (set `self.Mouse Save Ref` _asmouse_save)
    (else
      (bind _returnvalue_3 (`GameplayStatics.CreateSaveGameObject` "/Game/BluePrints/Saves/MouseSave.MouseSave_C"))
      (set `self.Mouse Save Ref` _returnvalue_3)))
  (add `/Game/BluePrints/Saves/MouseSave.UpdateSensitivity` (`self.Mouse Save Ref`) (delegate `UpdateSensititvity`))
  (`/Game/BluePrints/Saves/MouseSave.UpdateSensitivity` (`self.Mouse Save Ref`)))

(event `UpdateSensititvity`
  (set `self.MouseSensitivityX` (`/Game/BluePrints/Saves/MouseSave.MouseSensitivityX` (`self.Mouse Save Ref`)))
  (set `self.MouseSensitivityY` (`/Game/BluePrints/Saves/MouseSave.MouseSensitivityY` (`self.Mouse Save Ref`)))
  (set `self.InvertMouseSens` (select `bool` (`/Game/BluePrints/Saves/MouseSave.IsMouseInverted` (`self.Mouse Save Ref`)) :`false` 1.0 :`true` -1.0)))

(event `OnMoveInput`
  (params (InputX :type "Float (double-precision)") (InputY :type "Float (double-precision)"))
  (bind (_returnvalue_roll _returnvalue_pitch _returnvalue_yaw) (`KismetMathLibrary.BreakRotator` (`self.GetControlRotation`)))
  (bind (_returnvalue_roll_2 _returnvalue_pitch_2 _returnvalue_yaw_2) (`KismetMathLibrary.BreakRotator` (`self.GetControlRotation`)))
  (bind (_returnvalue_x _returnvalue_y) (`KismetMathLibrary.BreakVector` (`KismetMathLibrary.Normal` (`KismetMathLibrary.MakeVector` InputX InputY))))
  ; Get the direction the ball is supposed to move in
  (bind _output_get (set `self.Desired Velocity` (* (* _returnvalue_x (`self.MaxSpeed`)) (`KismetMathLibrary.GetRightVector` (`KismetMathLibrary.MakeRotator` 0.0 0.0 _returnvalue_yaw_2)))))
  ; Movement correction to prevent constant speed addition
  (bind _output_get_2 (set `self.Velocity Delta` (- _output_get (`self.GetVelocity`))))
  (if (< (`KismetMathLibrary.VSize` (`self.GetVelocity`)) (`self.VelocityThreshold`))
    (bind (_returnvalue_x_2 _returnvalue_y_2) (`KismetMathLibrary.BreakVector` (* _output_get_2 (`self.Acceleration`))))
    (`PrimitiveComponent.AddForce` (`self.Sphere`) (`KismetMathLibrary.MakeVector` _returnvalue_x_2 _returnvalue_y_2) "None" false)
    (bind _output_get_3 (set `self.Desired Velocity` (* (* _returnvalue_y (`self.MaxSpeed`)) (`KismetMathLibrary.GetForwardVector` (`KismetMathLibrary.MakeRotator` _returnvalue_roll 0.0 _returnvalue_yaw)))))
    (bind _output_get_4 (set `self.Velocity Delta` (- _output_get_3 (`self.GetVelocity`))))
    (if (< (`KismetMathLibrary.VSize` (`self.GetVelocity`)) (`self.VelocityThreshold`))
      (bind (_returnvalue_x_3 _returnvalue_y_3) (`KismetMathLibrary.BreakVector` (* _output_get_4 (`self.Acceleration`))))
      (`PrimitiveComponent.AddForce` (`self.Sphere`) (`KismetMathLibrary.MakeVector` _returnvalue_x_3 _returnvalue_y_3) "None" false))))

(event `OnPauseInput`
  (bind _returnvalue (`GameplayStatics.GetPlayerController` 0))
  (bind _options_widget_ref (`self.Options Widget Ref`)
    (:`then`
      (`Widget.RemoveFromParent` _options_widget_ref)
      (set `self.Options Widget Ref` null)
      (set `PlayerController.bShowMouseCursor` false _returnvalue)
      (`WidgetBlueprintLibrary.SetInputMode_GameOnly` _returnvalue))
    (:`else`
      (bind _returnvalue_2 (`|CreateWidget` "/Game/BluePrints/Widgets/W_Options.W_Options_C" null (`self.Mouse Save Ref`) self))
      (bind _output_get (set `self.Options Widget Ref` _returnvalue_2))
      (`UserWidget.AddToViewport` _output_get 0))))

(event `OnLookInput`
  (params (InputX :type "Float (double-precision)") (InputY :type "Float (double-precision)"))
  (`self.AddControllerYawInput` (* (`self.MouseSensitivityX`) (`self.InvertMouseSens`) InputX))
  (`self.AddControllerPitchInput` (* InputY (`self.MouseSensitivityY`) (`self.InvertMouseSens`))))

(event `OnJumpInput`
  (if (`self.isGrounded`)
    (`PrimitiveComponent.AddImpulse` (`self.Sphere`) (`KismetMathLibrary.MakeVector` 0.0 0.0 (`self.JumpHeight`)) "None" true)))

(fn `CheckGrounded`
  (bind _returnvalue (`self.K2_GetActorLocation`))
  (bind _outhit (`KismetSystemLibrary.LineTraceSingle` _returnvalue (- _returnvalue (0.0 0.0 70.0)) "TraceTypeQuery1"))
  (`/Engine/EditorBlueprintResources/StandardMacros.IsValid` (`.HitActor` (`GameplayStatics.BreakHitResult` _outhit))
    (:`Is Valid`
      (if (`self.ActorHasTag` (`.HitActor` (`GameplayStatics.BreakHitResult` _outhit)) "Ground")
        (set `self.isGrounded` true)))
    (:`Is Not Valid`
      (set `self.isGrounded` false))))

(fn `SimulateGravity`
  (bind (_returnvalue_x _returnvalue_y _returnvalue_z) (`KismetMathLibrary.BreakVector` (`SceneComponent.GetUpVector` (`self.Sphere`))))
  (if (not (`self.isGrounded`))
    (`PrimitiveComponent.AddForce` (`self.Sphere`) (`KismetMathLibrary.MakeVector` 0.0 0.0 (* (* _returnvalue_z -1.0) (`self.GravityMultiplier`) (`self.Delta Seconds`))) "None" true)))

(fn `UserConstructionScript`)