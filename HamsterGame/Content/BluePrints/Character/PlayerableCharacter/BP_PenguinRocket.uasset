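; BP_PenguinRocket is a playable penguin character that matches its animation to the current player state.
; OnPlayerStateChange switches on the state enum and plays a looping animation directly on the AnimalPinguin component: idle for Idle, walk for Walk, and run for Fireball.
; BeginPlay and Tick are disabled stubs, and the construction script only calls the parent.
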(event `self.OnPlayerStateChange`
  (params (CurE_PlayerStates :type "/Game/BluePrints/Character/Enums/E_PlayerStates Enum" :default "NewEnumerator0"))
  (switch `/Game/BluePrints/Character/Enums/E_PlayerStates` CurE_PlayerStates
    (:`NewEnumerator0`
      (`SkeletalMeshComponent.PlayAnimation` (`self.AnimalPinguin`) "/Game/Animals_Free/Animals/Animations/ANIM_Pinguin_001_Anim_Pinguin_001_idle.ANIM_Pinguin_001_Anim_Pinguin_001_idle" true))
    (:`NewEnumerator1`
      (`SkeletalMeshComponent.PlayAnimation` (`self.AnimalPinguin`) "/Game/Animals_Free/Animals/Animations/ANIM_Pinguin_001_Anim_Pinguin_001_walk.ANIM_Pinguin_001_Anim_Pinguin_001_walk" true))
    (:`NewEnumerator2`
      (`SkeletalMeshComponent.PlayAnimation` (`self.AnimalPinguin`) "/Game/Animals_Free/Animals/Animations/ANIM_Pinguin_001_Anim_Pinguin_001_run.ANIM_Pinguin_001_Anim_Pinguin_001_run" true))))

(fn `UserConstructionScript`
  (`parent.UserConstructionScript`))