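; Lobby pawn that registers the player with the lobby game state and opens the lobby menu.
; On BeginPlay it passes player controller 0's BP_PlayerStateLobby to GS_Lobby's AddPlayerToList, then shows W_LobbyMenu with Game and UI input and a visible cursor.
; Everything targets player index 0 rather than the pawn's own controller, and none of it runs if the GS_Lobby cast fails.
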(event `self.ReceiveBeginPlay`
  (bind _asgs_lobby (cast `/Game/BluePrints/GameState/GS_Lobby` (`GameplayStatics.GetGameState`)))
  (`/Game/BluePrints/GameState/GS_Lobby.AddPlayerToList` _asgs_lobby (cast `/Game/BluePrints/PlayerState/BP_PlayerStateLobby` (`Controller.PlayerState` (`GameplayStatics.GetPlayerController` 0)) :!pure true))
  (bind _returnvalue (`|CreateWidget` "/Game/BluePrints/Widgets/Lobby/W_LobbyMenu.W_LobbyMenu_C" (`GameplayStatics.GetPlayerController` 0)))
  (`UserWidget.AddToViewport` _returnvalue 0)
  (`WidgetBlueprintLibrary.SetInputMode_GameAndUIEx` (`GameplayStatics.GetPlayerController` 0) _returnvalue)
  (set `PlayerController.bShowMouseCursor` true (`GameplayStatics.GetPlayerController` 0)))

(fn `UserConstructionScript`)