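; Lobby player controller that gives the local player the lobby menu with mouse input and forwards lobby choices to the game state.
; On begin play it creates the widget and, with authority, shifts the first player pawn along X.
; RPC-named events toggle readiness on the player state, adjust GS_Lobby's ready count and set the selected map.
; Another event refreshes the player list; Tick debug-prints the game instance's selected character.
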(event `self.ReceiveTick`
  (params (DeltaSeconds :type "Float (single-precision)"))
  (if (`self.IsLocalController` self)
    (bind _asgi_hamster_game (cast `/Game/BluePrints/GameInstance/GI_HamsterGame` (`GameplayStatics.GetGameInstance`)))
    (`KismetSystemLibrary.PrintString` (`KismetSystemLibrary.GetClassDisplayName` (`/Game/BluePrints/GameInstance/GI_HamsterGame.SelectedCharacter` _asgi_hamster_game)) true true (struct :`R` 1.0 :`G` 0.072886 :`A` 1.0) DeltaSeconds)))

(event `self.ReceiveBeginPlay`
  (bind _returnvalue (`GameplayStatics.GetPlayerPawn` 0))
  (bind _returnvalue_location (`KismetMathLibrary.BreakTransform` (`self.GetTransform` _returnvalue)))
  (if (`self.IsLocalController` self)
    (`|ExecutionSequence`
      (:`then_0`
        (bind _returnvalue_2 (`|CreateWidget` "/Game/BluePrints/Widgets/Lobby/W_LobbyMenu.W_LobbyMenu_C" self))
        (bind _output_get (set `self.Lobby Menu` _returnvalue_2))
        (`UserWidget.AddToViewport` _output_get 0)
        (`WidgetBlueprintLibrary.SetInputMode_GameAndUIEx` (`GameplayStatics.GetPlayerController` 0) _returnvalue_2)
        (set `PlayerController.bShowMouseCursor` true (`GameplayStatics.GetPlayerController` 0)))
      (:`then_1`
        (if (`self.HasAuthority` (`GameplayStatics.GetPlayerPawn` 0))
          (`self.K2_SetActorLocation` _returnvalue (+ _returnvalue_location (-1000.0 0.0 0.0)) false false))))))

(event `RPC_AddReadyToServer`
  (bind _asbp_player_state_lobby (cast `/Game/BluePrints/PlayerState/BP_PlayerStateLobby` (`self.PlayerState`)))
  (`/Game/BluePrints/PlayerState/BP_PlayerStateLobby.UpdateReadyState` _asbp_player_state_lobby)
  (bind _asgs_lobby (cast `/Game/BluePrints/GameState/GS_Lobby` (`GameplayStatics.GetGameState`)))
  (`/Game/BluePrints/GameState/GS_Lobby.RPC_Set Amount Of Readys` _asgs_lobby (+ (`/Game/BluePrints/GameState/GS_Lobby.AmountOfReadys` _asgs_lobby) (`KismetMathLibrary.SelectInt` 1 -1 (`/Game/BluePrints/PlayerState/BP_PlayerStateLobby.IsReady` _asbp_player_state_lobby)))))

(event `RPC_SelectMap`
  (params (MapPath :type String))
  (bind _asgs_lobby (cast `/Game/BluePrints/GameState/GS_Lobby` (`GameplayStatics.GetGameState`)))
  (`/Game/BluePrints/GameState/GS_Lobby.SetSelectedLevel` _asgs_lobby MapPath))

(event `UpdatePlayerInfoUI`
  (`/Game/BluePrints/Widgets/Lobby/W_LobbyPlayerInfo.UpdatePlayerInfoList` (`/Game/BluePrints/Widgets/Lobby/W_LobbyMenu.W_LobbyPlayerInfo` (`self.Lobby Menu`))))

(fn `UserConstructionScript`)