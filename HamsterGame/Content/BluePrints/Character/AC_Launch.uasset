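; AC_Launch is a component that knocks a hit target away by overwriting the hit component's physics linear velocity.
; LaunchCharacter stores the hit data, then multiplies GetDirectionOfLaunch by negated LaunchStrength.
; With TrueKnockback, unless the owner is the instigator, strength also scales with the hit player's 1v1 KnockbackPercent.
; KnocbackMultiplier is stored but unused, and GetDirectionOfLaunch's causer-to-target plus UpVector calculation appears unconnected.
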(event `LaunchCharacter`
  (params (Causer :type "Actor Object Reference") (Instigator :type "Actor Object Reference") (HitActor :type "Actor Object Reference") (HitComponent :type "PrimitiveComponent Object Reference") (UpVector :type "Vector Structure") (LaunchStrength :type "Float (double-precision)") (KnocbackMultiplier :type "Float (double-precision)") (TrueKnocback :type Boolean))
  (set `self.Causer` Causer)
  (set `self.Instigator` Instigator)
  (set `self.Hit Actor` HitActor)
  (set `self.Hit Component` HitComponent)
  (set `self.Up Vector` UpVector)
  (set `self.Launch Strength` LaunchStrength)
  (set `self.Knocback Multiplier` KnocbackMultiplier)
  (if (== (`self.GetOwner`) (`self.Instigator`))
    (`PrimitiveComponent.SetPhysicsLinearVelocity` (`self.Hit Component`) (* (`self.GetDirectionOfLaunch`) (`self.Launch Strength`) -1.0) false "None" :!label _label)
    (elif TrueKnocback
      (`PrimitiveComponent.SetPhysicsLinearVelocity` (`self.Hit Component`) (* (`self.GetDirectionOfLaunch`) (`self.Launch Strength`) (/ (+ (`/Game/BluePrints/PlayerState/BP_1v1PlayerState.KnockbackPercent` (cast `/Game/BluePrints/PlayerState/BP_1v1PlayerState` (`Controller.PlayerState` (`Pawn.GetController` (cast `/Game/BluePrints/Character/BP_BasePlayerPawn` (`self.Hit Actor`) :!pure true))) :!pure true)) 100.0) 100.0) -1.0) false "None")
      (else
        (goto _label)))))