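; Lobby player state that holds a player's ready flag, selected character and team choice before a 1v1 match.
; CopyProperties carries the character and team selection into BP_1v1PlayerState when the player state is replaced, as in seamless travel.
; UpdateReadyState toggles IsReady, whose OnRep handler is empty.
; A Test event asks the lobby controller to refresh its player info UI.
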(event `Test`
  (bind _asbp_lobby_controller (cast `/Game/BluePrints/Character/BP_LobbyController` (`self.GetPlayerController`)))
  (`/Game/BluePrints/Character/BP_LobbyController.UpdatePlayerInfoUI` _asbp_lobby_controller))

(event `self.ReceiveCopyProperties`
  (params (NewPlayerState :type "PlayerState Object Reference"))
  (bind _asbp_1v_1player_state (cast `/Game/BluePrints/PlayerState/BP_1v1PlayerState` NewPlayerState))
  (set `/Game/BluePrints/PlayerState/BP_1v1PlayerState.SelectedCharacter` (`self.SelectedCharacter`) _asbp_1v_1player_state)
  (set `/Game/BluePrints/PlayerState/BP_1v1PlayerState.IsOnRedTeam` (`self.IsOnRedTeam`) _asbp_1v_1player_state))

(fn `OnRep_IsReady`)

(fn `UpdateReadyState`
  (set `self.IsReady` (not (`self.IsReady`))))

(fn `UserConstructionScript`)