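; Game State for the 1v1 mode that tracks the match timer, players and red/blue teams.
; Tick counts down TimeRemaining and ends the match once at zero, as a draw if both teams still have lives.
; CheckIfMatchOver ends it early when HasTeamWon finds the match decided.
; OnRep functions, RPCs and event dispatchers push timer, roster, player info and match results to the UI and other listeners.
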(event `self.ReceiveBeginPlay`
  ; Timer logic
  (set `self.TimeRemaining` (`self.MaxTimeInSeconds`)))

(event `self.ReceiveTick`
  (params (DeltaSeconds :type "Float (single-precision)"))
  ; Timer logic
  (bind _output_get (set `self.TimeRemaining` (- (`self.TimeRemaining`) DeltaSeconds)))
  (if (<= _output_get 0.0)
    (`/Engine/EditorBlueprintResources/StandardMacros.DoOnce` false
      (:`Completed`
        (`self.EndMatchByTimer`)))))

(event `CheckIfMatchOver`
  (bind (_matchstillongoing _hasredteamwon_) (`self.HasTeamWon`))
  (if (not _matchstillongoing)
    (`self.EndMatchLogic` _hasredteamwon_)))

(event `CallUpdateTimer`
  ; Timer logic
  (`self.UpdateTimer`))

(event `EndMatchByTimer`
  (bind (_matchstillongoing _hasredteamwon_) (`self.HasTeamWon`))
  (`self.EndMatchLogic` _hasredteamwon_ _matchstillongoing))

(event `RPC_EndMatchByTimer`)

(event `UpdatePlayersInfo`
  (params (PlayerState :type "/Game/BluePrints/PlayerState/BP_1v1PlayerState Object Reference"))
  ; Update Players Info
  (`self.UpdatePlayerInfo` (`AdvancedSessionsLibrary.GetUniqueNetIDFromPlayerState` PlayerState))
  (`self.Server_UpdatePlayerInfo` PlayerState))

(event `EndMatchLogic`
  (params (`HasRedTeamWon?` :type Boolean) (`IsMatchDraw?` :type Boolean))
  (`self.EndOfMatch` `HasRedTeamWon?` `IsMatchDraw?`)
  (`self.RPC_EndMatchLogic` `HasRedTeamWon?` `IsMatchDraw?`))

(event `Server_UpdatePlayerInfo`
  (params (`Player State` :type "/Game/BluePrints/PlayerState/BP_1v1PlayerState Object Reference"))
  ; Update Players Info
  (`self.UpdatePlayerInfo` (`AdvancedSessionsLibrary.GetUniqueNetIDFromPlayerState` `Player State`)))

(event `RPC_EndMatchLogic`
  (params (HasRedTeamWon :type Boolean) (IsMatchDraw :type Boolean))
  (`self.EndOfMatch` HasRedTeamWon IsMatchDraw))

(event `AddNewPlayer`
  (params (`New Player` :type "/Game/BluePrints/PlayerState/BP_1v1PlayerState Object Reference"))
  ; Add and Initialize players to UI
  (`/Game/BluePrints/Character/BP_Base_PlayerController.InitializeTeamsUI` (cast `/Game/BluePrints/Character/BP_Base_PlayerController` (`PlayerState.GetPlayerController` `New Player`) :!pure true))
  (`self.AssignPlayerTeam` `New Player`)
  (`KismetArrayLibrary.Array_Add` (`self.PlayerStates`) `New Player`)
  (`self.Server_CallAddNewPlayer`))

(event `Server_CallAddNewPlayer`
  ; Add and Initialize players to UI
  (`self.AddPlayerToUI`))

(event `InitializeTeam UI`
  (params (`New player` :type "/Game/BluePrints/PlayerState/BP_1v1PlayerState Object Reference"))
  ; Add and Initialize players to UI
  (`/Engine/EditorBlueprintResources/StandardMacros.IsValid` `New player`
    (:`Is Valid`
      (`/Game/BluePrints/Character/BP_Base_PlayerController.InitializeTeamsUI` (cast `/Game/BluePrints/Character/BP_Base_PlayerController` (`PlayerState.GetPlayerController` `New player`) :!pure true)))))

(event `AssignPlayerTeam`
  (params (Player :type "/Game/BluePrints/PlayerState/BP_1v1PlayerState Object Reference"))
  ; Add and Initialize players to UI
  (if (`/Game/BluePrints/PlayerState/BP_1v1PlayerState.IsOnRedTeam` Player)
    (`KismetArrayLibrary.Array_Add` (`self.Red Team Players`) Player)
    (else
      (`KismetArrayLibrary.Array_Add` (`self.Blue Team Players`) Player))))

(fn `GetPlayerStateByUniqeNetID`
  (params (UniqueNetID :type "BPUniqueNetId Structure"))
  (returns (PlayerState :type "/Game/BluePrints/PlayerState/BP_1v1PlayerState Object Reference"))
  (for _array_element (`self.PlayerStates`)
    (if (== (`AdvancedSessionsLibrary.GetUniqueNetIDFromPlayerState` _array_element) UniqueNetID)
      (return _array_element))))

(fn `HasTeamWon`
  (returns (MatchStillOngoing :type Boolean) (`HasRedTeamWon?` :type Boolean))
  (locals (HasRedTeamWon :type Boolean :default false) (HasBlueTeamWon :type Boolean :default false))
  (bind _hasredteamwon (`local.HasRedTeamWon`))
  (for _array_element (`self.Red Team Players`)
    (if (> (`/Game/BluePrints/PlayerState/BP_1v1PlayerState.livesRemaining` _array_element) 0)
      (set `local.HasRedTeamWon` true)))
  (for _array_element_2 (`self.Blue Team Players`)
    (if (> (`/Game/BluePrints/PlayerState/BP_1v1PlayerState.livesRemaining` _array_element_2) 0)
      (set `local.HasBlueTeamWon` true)))
  (return (and (`local.HasBlueTeamWon`) _hasredteamwon) _hasredteamwon))

(fn `OnRep_PlayerStates`
  (bind _playerstates (`self.PlayerStates`))
  (`self.InitializeTeam UI` (`|GetArrayItem` _playerstates (`KismetArrayLibrary.Array_LastIndex` _playerstates)))
  (`self.AddPlayerToUI`))

(fn `OnRep_TimeRemaining`
  (`self.UpdateTimer`))

(fn `UserConstructionScript`)