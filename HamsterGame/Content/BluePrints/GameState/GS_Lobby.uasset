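; Lobby GameState that tracks the player list, player and ready counts, and selected level, and starts the match when everyone is ready.
; RepNotify functions and setter events fire update calls for player info, counts and map selection.
; A ready-count change also checks each player's IsReady and compares ready to player totals.
; When both pass, it sends the selected level to BP_LobbyGameMode's SendToMap.
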(event `SendToMatch`
  (bind _asbp_lobby_game_mode (cast `/Game/BluePrints/GameMode/BP_LobbyGameMode` (`GameplayStatics.GetGameMode`)))
  (`/Game/BluePrints/GameMode/BP_LobbyGameMode.SendToMap` _asbp_lobby_game_mode (`self.SelectedLevel`)))

(event `SetSelectedLevel`
  (params (SelectedLevel :type String))
  (set `self.SelectedLevel` SelectedLevel)
  (set `self.HasSelectedMap` true)
  (`self.UpdateMapSelected`))

(event `RPC_Set Amount Of Readys`
  (params (AmountOfReadys :type Integer))
  (set `self.AmountOfReadys` AmountOfReadys)
  (`KismetSystemLibrary.PrintString` "3")
  (`self.UpdateAmountOfReadys`))

(event `UpdateInfoPlayers`
  (`self.UpdateAmountOfPlayers`)
  (`self.UpdatePlayerInfoUI`))

(fn `AddPlayerToList`
  (params (NewPlayer :type "/Game/BluePrints/PlayerState/BP_PlayerStateLobby Object Reference"))
  (`KismetArrayLibrary.Array_AddUnique` (`self.AllPlayers`) NewPlayer))

(fn `CheckAllReadyThenSendToMap`
  (locals (`AreAllReady?` :type Boolean :default true))
  (bind _players_states (`self.GetAllPlayers`))
  (for _array_element _players_states
    (if (not (`/Game/BluePrints/PlayerState/BP_PlayerStateLobby.IsReady` _array_element))
      (set `local.AreAllReady?` false)))
  (if (`local.AreAllReady?`)
    (if (>= (`self.AmountOfReadys`) (`self.AmountOfPlayers`))
      (`self.SendToMatch`))))

(fn `GetAllPlayers`
  (returns (`Players States` :type "Array of /Game/BluePrints/PlayerState/BP_PlayerStateLobby Object Reference"))
  (return (`self.AllPlayers`)))

(fn `GetPlayerStateByUniqueNetID`
  (params (PlayerNetID :type "BPUniqueNetId Structure"))
  (returns (PlayerState :type "/Game/BluePrints/PlayerState/BP_PlayerStateLobby Object Reference"))
  (for _array_element (`self.AllPlayers`)
    (if (== (`AdvancedSessionsLibrary.GetUniqueNetIDFromPlayerState` _array_element) PlayerNetID)
      (return _array_element))))

(fn `OnRep_AllPlayers`
  (`self.UpdatePlayerInfoUI`))

(fn `OnRep_AmountOfPlayers`
  (`self.UpdateAmountOfPlayers`))

(fn `OnRep_AmountOfReadys`
  (`KismetSystemLibrary.PrintString` "4")
  (`self.UpdateAmountOfReadys`)
  (`self.CheckAllReadyThenSendToMap`))

(fn `OnRep_SelectedLevel`
  (set `self.HasSelectedMap` true)
  (`self.UpdateMapSelected`))

(fn `RemovePlayerFromList`
  (params (RemovedPlayer :type "/Game/BluePrints/PlayerState/BP_PlayerStateLobby Object Reference"))
  (`KismetArrayLibrary.Array_RemoveItem` (`self.AllPlayers`) RemovedPlayer))

(fn `SetAmountOfReadys`
  (params (Input :type Integer))
  (set `self.AmountOfReadys` Input))

(fn `UserConstructionScript`)