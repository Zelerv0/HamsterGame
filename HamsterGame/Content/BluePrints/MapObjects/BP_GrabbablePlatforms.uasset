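; Map object platform that a grappling hook can grab only briefly before it drops the grapple and goes inactive.
; Hook overlap with the HitBox turns the dynamic material yellow and starts a timer to disable the platform, cancelling the grapple, turning red and switching off collision.
; End overlap disables it immediately and starts a timer that restores green and query-only collision.
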(event `self.ReceiveBeginPlay`
  (bind _returnvalue (`PrimitiveComponent.CreateDynamicMaterialInstance` (`self.Platform`) 0 null "None"))
  (set `self.Dynamic Material` _returnvalue))

(event `StartTimer`
  (params (FunctionName :type String) (Time :type "Float (single-precision)"))
  (`KismetSystemLibrary.K2_SetTimer` null FunctionName Time))

(event `self.HitBox.OnComponentBeginOverlap`
  (params (OverlappedComponent :type "PrimitiveComponent Object Reference") (OtherActor :type "Actor Object Reference") (OtherComp :type "PrimitiveComponent Object Reference") (OtherBodyIndex :type Integer) (bFromSweep :type Boolean) (SweepResult :type "HitResult Structure (by ref)"))
  (bind _asbp_grappling_hook (cast `/Game/BluePrints/Projectile/BP_GrapplingHook` OtherActor))
  (set `self.As BP Grappling Hook` _asbp_grappling_hook)
  (`self.SetWarningState`)
  (`self.StartTimer` "DisablePlatform" (`self.SecondsToDisable`)))

(event `SetWarningState`
  (`MaterialInstanceDynamic.SetVectorParameterValue` (`self.Dynamic Material`) (`self.Parameter Name`) (`self.YellowColor`)))

(event `DisablePlatform`
  (`/Game/BluePrints/Projectile/BP_GrapplingHook.CancelGrapple` (`self.As BP Grappling Hook`))
  (`MaterialInstanceDynamic.SetVectorParameterValue` (`self.Dynamic Material`) (`self.Parameter Name`) (`self.RedColor`))
  (`PrimitiveComponent.SetCollisionEnabled` (`self.CollisionBox`) "NoCollision")
  (`PrimitiveComponent.SetCollisionEnabled` (`self.HitBox`) "NoCollision"))

(event `self.HitBox.OnComponentEndOverlap`
  (params (OverlappedComponent :type "PrimitiveComponent Object Reference") (OtherActor :type "Actor Object Reference") (OtherComp :type "PrimitiveComponent Object Reference") (OtherBodyIndex :type Integer))
  (cast `/Game/BluePrints/Projectile/BP_GrapplingHook` OtherActor)
  (`self.DisablePlatform`)
  (`self.StartTimer` "EnablePlatform" (`self.SecondsToEnable`)))

(event `EnablePlatform`
  (`MaterialInstanceDynamic.SetVectorParameterValue` (`self.Dynamic Material`) (`self.Parameter Name`) (`self.GreenColor`))
  (`PrimitiveComponent.SetCollisionEnabled` (`self.CollisionBox`) "QueryOnly")
  (`PrimitiveComponent.SetCollisionEnabled` (`self.HitBox`) "QueryOnly"))

(fn `UserConstructionScript`)