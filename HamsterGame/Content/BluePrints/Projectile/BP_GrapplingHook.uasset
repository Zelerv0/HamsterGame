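; Grappling hook projectile fired by BP_BasePlayerPawn, with a cable attached to the player's shot point through OnRep_OwningPlayer.
; A looping timer updates cable length; reaching max distance disables collision, resets velocity via ReturnVelocity and destroys the hook after a delay.
; A hit sets Anchor state and records rope length.
; While anchored, Tick constrains the player's physics sphere, stripping outward velocity and applying spring force for a swing; pull state is empty.
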(event `self.ReceiveTick`
  (params (DeltaSeconds :type "Float (single-precision)"))
  (set `self.Delta Seconds` DeltaSeconds)
  (switch `/Game/BluePrints/Character/Enums/E_GrappleHookStates` (`/Game/BluePrints/Character/BP_BasePlayerPawn.CurE_GrappleState` (`self.OwningPlayer`))
    (:`NewEnumerator0`
      (`self.OnAnchorState`))))

(event `self.ReceiveBeginPlay`
  (bind _asbp_base_player_pawn (cast `/Game/BluePrints/Character/BP_BasePlayerPawn` (`self.GetOwner`)))
  (set `self.OwningPlayer` _asbp_base_player_pawn)
  (`self.Grapple`))

(event `CancelGrapple`
  (`self.DestroyGrapple`))

(event `Grapple`
  (set `self.MaxGrappleDistance` (`/Game/BluePrints/Character/BP_BasePlayerPawn.GrappleDistance` (`self.OwningPlayer`)))
  (bind _returnvalue (`KismetSystemLibrary.K2_SetTimerDelegate` (delegate `UpdateCableVisuals`) 0.001 true))
  (set `self.TimerUpdateVisuals` _returnvalue))

(event `UpdateCableVisuals`
  (`self.SetCableLength`)
  (if (>= (`CableComponent.CableLength` (`self.Cable`)) (`self.MaxGrappleDistance`))
    (`/Engine/EditorBlueprintResources/StandardMacros.DoOnce` false
      (:`Completed`
        (set `MovementComponent.Velocity` (`self.ReturnVelocity`) (`self.ProjectileMovement`))
        (`PrimitiveComponent.SetCollisionEnabled` (`self.Sphere`) "NoCollision")
        (`KismetSystemLibrary.Delay` 0.5)
        (`self.CancelGrapple`)
        (set `/Game/BluePrints/Character/BP_BasePlayerPawn.CurE_GrappleState` "NewEnumerator2" (`self.OwningPlayer`))))))

(event `self.Sphere.OnComponentHit`
  (params (HitComponent :type "PrimitiveComponent Object Reference") (OtherActor :type "Actor Object Reference") (OtherComp :type "PrimitiveComponent Object Reference") (NormalImpulse :type "Vector Structure") (Hit :type "HitResult Structure (by ref)"))
  (`self.GrappleHit` Hit_Location))

(event `GrappleHit`
  (params (GrapplePoint :type "Vector Structure"))
  (set `self.GrapplePoint` GrapplePoint)
  (set `self.Hit Distance` (`KismetMathLibrary.VSize` (- (`SceneComponent.K2_GetComponentLocation` (`/Game/BluePrints/Character/BP_BasePlayerPawn.Sphere` (`self.OwningPlayer`))) (`self.GrapplePoint`))))
  (`/Game/BluePrints/Character/BP_BasePlayerPawn.SetGrappleState` (`self.OwningPlayer`) "NewEnumerator0"))

(event `OnAnchorState`
  (bind _owningplayer (`self.OwningPlayer`))
  (bind _dir (`self.Dir`))
  (bind _returnvalue (`self.GetVelocity` (`self.OwningPlayer`)))
  (bind _sphere (`/Game/BluePrints/Character/BP_BasePlayerPawn.Sphere` (`self.OwningPlayer`)))
  (bind _returnvalue_2 (- (`SceneComponent.K2_GetComponentLocation` (`/Game/BluePrints/Character/BP_BasePlayerPawn.Sphere` _owningplayer)) (`self.GrapplePoint`)))
  (set `self.Distance` (`KismetMathLibrary.VSize` _returnvalue_2))
  (bind _output_get (set `self.Dir` (`KismetMathLibrary.Normal` _returnvalue_2)))
  (set `self.OutwardSpeed` (`KismetMathLibrary.Dot_VectorVector` (`self.GetVelocity` _owningplayer) _output_get))
  (bind _output_get_2 (set `self.RadialVelocity` (* _dir (`KismetMathLibrary.Dot_VectorVector` _dir _returnvalue))))
  (bind _output_get_3 (set `self.TangentalVelocity` (- _returnvalue _output_get_2)))
  (if (and (> (`self.OutwardSpeed`) 0.0) (>= (`self.Distance`) (`self.Hit Distance`)))
    (`PrimitiveComponent.SetPhysicsLinearVelocity` _sphere _output_get_3 false "None")
    (if (>= (`self.Distance`) (`self.Hit Distance`))
      (`PrimitiveComponent.AddForce` _sphere (* (`self.Dir`) (- (`self.Hit Distance`) (`self.Distance`)) 1000.0) "None" true))))

(event `OnPullState`)

(fn `DestroyGrapple`
  (`KismetSystemLibrary.K2_ClearAndInvalidateTimerHandle` (`self.TimerUpdateVisuals`))
  (`self.K2_DestroyActor`)
  (set `/Game/BluePrints/Character/BP_BasePlayerPawn.IsGrappled` false (`self.OwningPlayer`)))

(fn `OnRep_OwningPlayer`
  (bind _owningplayer (`self.OwningPlayer`))
  (`CableComponent.SetAttachEndTo` (`self.Cable`) _owningplayer (`KismetStringLibrary.Conv_StringToName` (`KismetSystemLibrary.GetObjectName` (`/Game/BluePrints/Character/BP_BasePlayerPawn.ShotPoint` _owningplayer))) "None"))

(fn `SetCableLength`
  (set `CableComponent.CableLength` (`KismetMathLibrary.Vector_Distance` (`self.K2_GetActorLocation` (`self.OwningPlayer`)) (`SceneComponent.K2_GetComponentLocation` (`self.StaticMesh`))) (`self.Cable`)))

(fn `UserConstructionScript`)