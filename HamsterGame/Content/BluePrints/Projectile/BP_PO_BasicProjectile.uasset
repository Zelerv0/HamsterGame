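; BP_PO_BasicProjectile is a basic projectile Blueprint that deals damage on impact.
; On Hit, it spawns an actor of a configurable class at the impact location, owned by the projectile's owner.
; Actors tagged "Damagable" take KnockbackDMG through ApplyDamage, credited to the owner's instigator controller.
; It then calls the parent Hit logic; BeginPlay and the overlap event add no behavior.
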(event `self.ReceiveBeginPlay`)

(event `self.ReceiveHit`
  (params (MyComp :type "PrimitiveComponent Object Reference") (Other :type "Actor Object Reference") (OtherComp :type "PrimitiveComponent Object Reference") (bSelfMoved :type Boolean) (HitLocation :type "Vector Structure") (HitNormal :type "Vector Structure") (NormalImpulse :type "Vector Structure") (Hit :type "HitResult Structure (by ref)"))
  (set `self.Hit Normal` HitNormal)
  (`|SpawnActorFromClass` (`self.Class`) (`KismetMathLibrary.MakeTransform` (`.Location` (`GameplayStatics.BreakHitResult` Hit))) "Undefined" "MultiplyWithRoot" (`self.GetOwner`) null)
  (if (`self.ActorHasTag` Other "Damagable")
    (`GameplayStatics.ApplyDamage` Other (`self.KnockbackDMG`) (`self.GetInstigatorController` (`self.GetOwner`)) self "/Script/Engine.DamageType"))
  (`parent.ReceiveHit` null null null false (0.0 0.0 0.0) (0.0 0.0 0.0) (0.0 0.0 0.0) Hit))

(fn `UserConstructionScript`
  (`parent.UserConstructionScript`))