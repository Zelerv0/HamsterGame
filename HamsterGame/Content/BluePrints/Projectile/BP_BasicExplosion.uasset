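; BP_BasicExplosion is a short-lived explosion actor that knocks back player pawns and deals damage within its sphere, destroying itself after its lifetime.
; On sphere overlap, it replaces the BP_BasePlayerPawn physics sphere's velocity with a scaled launch away from the blast center, biased along the explosion's up vector.
; The owner still gets launched but takes no damage; damage to other actors is credited to the owner's instigator controller.
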(event `self.ReceiveBeginPlay`
  (`KismetSystemLibrary.K2_SetTimerDelegate` (delegate `DestroyOnEndLifetime`) (`self.LifeTime`)))

(event `DestroyOnEndLifetime`
  (`self.K2_DestroyActor`))

(event `self.Sphere.OnComponentBeginOverlap`
  (params (OverlappedComponent :type "PrimitiveComponent Object Reference") (OtherActor :type "Actor Object Reference") (OtherComp :type "PrimitiveComponent Object Reference") (OtherBodyIndex :type Integer) (bFromSweep :type Boolean) (SweepResult :type "HitResult Structure (by ref)"))
  (set `self.HitComponent` OtherComp)
  (bind _output_get (set `self.OverlappedActor` OtherActor))
  (`PrimitiveComponent.SetPhysicsLinearVelocity` (`/Game/BluePrints/Character/BP_BasePlayerPawn.Sphere` (cast `/Game/BluePrints/Character/BP_BasePlayerPawn` (`self.OverlappedActor`) :!pure true)) (* (`KismetMathLibrary.Normal` (+ (- (`self.K2_GetActorLocation` _output_get) (`SceneComponent.K2_GetComponentLocation` (`self.Sphere`))) (`self.GetActorUpVector`))) (`self.LaunchStrength`) (`self.LaunchMult`)) false "None")
  (if (not (== (`self.OverlappedActor`) (`self.GetOwner`)))
    (`GameplayStatics.ApplyDamage` (`self.OverlappedActor`) (`self.Damage`) (`self.GetInstigatorController` (`self.GetOwner`)) self)))

(fn `UserConstructionScript`)